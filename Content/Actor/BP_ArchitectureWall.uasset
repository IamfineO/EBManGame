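; BP_ArchitectureWall is an actor that builds a straight wall by repeating one static mesh from its origin toward an EndPoint vector.
; Its construction script divides the EndPoint distance by Width, truncates the result, and adds a mesh component at each step, including both zero and the last index.
; Each segment sits Width apart along the normalized direction and rotates its X axis to face along it.
; The event graph holds no active logic.
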(fn `UserConstructionScript`
  (bind _endpoint (`self.EndPoint`))
  (for _index (range (+ (`KismetMathLibrary.FTrunc` (/ (`KismetMathLibrary.VSize` _endpoint) (`self.Width`))) 1))
    (bind _returnvalue (`AddComponent|NODE_AddStaticMeshComponent-0` :`RelativeTransform` (`KismetMathLibrary.MakeTransform` (* (* (`KismetMathLibrary.Normal` _endpoint) _index) (`self.Width`)) (`KismetMathLibrary.Conv_VectorToRotator` _endpoint))))
    (`StaticMeshComponent.SetStaticMesh` _returnvalue (`self.Mesh`))))