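; BP_BorderWall is an actor that builds a rectangular border wall from repeated copies of one mesh.
; The construction script places a mesh at the origin, divides EndPoint's X and Y by Width, and truncates to get tile counts.
; Two loops add separate, unrotated static mesh components along opposite edge pairs, overlapping at the far corner.
; The event graph has no active logic.
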(fn `UserConstructionScript`
  (bind (_endpoint_x _endpoint_y) (`KismetMathLibrary.BreakVector` (`self.EndPoint`)))
  (bind _width (`self.Width`))
  (`|ExecutionSequence`
    (:`then_0`
      (bind _returnvalue (`AddComponent|NODE_AddStaticMeshComponent-4`))
      (`StaticMeshComponent.SetStaticMesh` _returnvalue (`self.Mesh`)))
    (:`then_1`
      (set `self.XSum` (`KismetMathLibrary.FTrunc` (/ _endpoint_x _width)))
      (set `self.YSum` (`KismetMathLibrary.FTrunc` (/ _endpoint_y _width)))
      (for _index (range 1 (+ (`self.XSum`) 1))
        (bind _returnvalue_2 (* _index (`self.Width`)))
        ;[1 1 1] x轴方向沿原点
        (bind _returnvalue_3 (`AddComponent|NODE_AddStaticMeshComponent-0` :`RelativeTransform` (`KismetMathLibrary.MakeTransform` (`KismetMathLibrary.MakeVector` _returnvalue_2))))
        (`StaticMeshComponent.SetStaticMesh` _returnvalue_3 (`self.Mesh`))
        ;[1 1 1] x轴方向沿对边方向
        (bind _returnvalue_4 (`AddComponent|NODE_AddStaticMeshComponent-1` :`RelativeTransform` (`KismetMathLibrary.MakeTransform` (`KismetMathLibrary.MakeVector` _returnvalue_2 (* (`self.YSum`) (`self.Width`))))))
        (`StaticMeshComponent.SetStaticMesh` _returnvalue_4 (`self.Mesh`)))
      (for _index_2 (range 1 (+ (`self.YSum`) 1))
        (bind _returnvalue_5 (* _index_2 (`self.Width`)))
        ;[1 1 1] y轴方向沿原点
        (bind _returnvalue_6 (`AddComponent|NODE_AddStaticMeshComponent-2` :`RelativeTransform` (`KismetMathLibrary.MakeTransform` (`KismetMathLibrary.MakeVector` 0.0 _returnvalue_5))))
        (`StaticMeshComponent.SetStaticMesh` _returnvalue_6 (`self.Mesh`))
        ;[1 1 1] y轴方向沿对边方向
        (bind _returnvalue_7 (`AddComponent|NODE_AddStaticMeshComponent-3` :`RelativeTransform` (`KismetMathLibrary.MakeTransform` (`KismetMathLibrary.MakeVector` (* (`self.XSum`) (`self.Width`)) _returnvalue_5))))
        (`StaticMeshComponent.SetStaticMesh` _returnvalue_7 (`self.Mesh`))))))